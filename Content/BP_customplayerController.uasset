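; Player controller that turns Enhanced Input actions into jump, move, look and door interaction for player character 0.
; It adds the Imc_Player mapping context on BeginPlay.
; Movement follows the BP_Player camera's yaw, while look input drives controller yaw and pitch.
; Interact runs a short, debug-drawn visibility trace forward from the camera and calls OpenDoor on any BP_Door hit.
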(event Input|EnhancedActionEvents|EnhancedInputActionIA_Jump
  (params (ActionValue :type Boolean) (ElapsedSeconds :type Float%20%28double-precision%29) (TriggeredSeconds :type Float%20%28double-precision%29) (InputAction :type Input%20Action%20Object%20Reference :default "/Game/Inputs/Action/IA_Jump.IA_Jump"))
  (:Started
    (Character|Jump (Game|GetPlayerCharacter 0))))

(event Input|EnhancedActionEvents|EnhancedInputActionIA_Move
  (params (ActionValue :type Vector%202D%20Structure) (ElapsedSeconds :type Float%20%28double-precision%29) (TriggeredSeconds :type Float%20%28double-precision%29) (InputAction :type Input%20Action%20Object%20Reference :default "/Game/Inputs/Action/IA_Move.IA_Move"))
  (bind _returnvalue (Game|GetPlayerCharacter 0))
  (:Triggered
    (bind _asbp_player (Utilities|Casting|CastToBP_Player _returnvalue))
    (Pawn|Input|AddMovementInput _returnvalue (Math|Vector|GetForwardVector (Math|Rotator|MakeRotator 0.0 0.0 (.yaw (Transformation|GetWorldRotation (Variables|/Game/BP_Player.BP_Player_C|GetCamera _asbp_player))))) (.x ActionValue) false)
    (Pawn|Input|AddMovementInput _returnvalue (Math|Vector|GetRightVector (Math|Rotator|MakeRotator 0.0 0.0 (.yaw (Transformation|GetWorldRotation (Variables|/Game/BP_Player.BP_Player_C|GetCamera _asbp_player))))) (.y ActionValue) false)))

(event Input|EnhancedActionEvents|EnhancedInputActionIA_Look
  (params (ActionValue :type Vector%202D%20Structure) (ElapsedSeconds :type Float%20%28double-precision%29) (TriggeredSeconds :type Float%20%28double-precision%29) (InputAction :type Input%20Action%20Object%20Reference :default "/Game/Inputs/Action/IA_Look.IA_Look"))
  (bind _returnvalue (Game|GetPlayerCharacter 0))
  (:Triggered
    (Pawn|Input|AddControllerYawInput _returnvalue (.x ActionValue))
    (Pawn|Input|AddControllerPitchInput _returnvalue (.y ActionValue))))

(event Input|EnhancedActionEvents|EnhancedInputActionIA_Interact
  (params (ActionValue :type Boolean) (ElapsedSeconds :type Float%20%28double-precision%29) (TriggeredSeconds :type Float%20%28double-precision%29) (InputAction :type Input%20Action%20Object%20Reference :default "/Game/Inputs/Action/IA_Interact.IA_Interact"))
  (:Triggered
    (bind _asbp_player (Utilities|Casting|CastToBP_Player (Game|GetPlayerCharacter 0)))
    (bind _outhit (Collision|LineTraceByChannel (Transformation|GetWorldLocation (Variables|/Game/BP_Player.BP_Player_C|GetCamera _asbp_player)) (+ (Transformation|GetWorldLocation (Variables|/Game/BP_Player.BP_Player_C|GetCamera _asbp_player)) (* (Math|Vector|GetForwardVector (Variables|/Game/BP_Player.BP_Player_C|GetCamera _asbp_player)) 2e+02)) "TraceTypeQuery1" false 0 "ForDuration"))
    (bind _asbp_door (Utilities|Casting|CastToBP_Door (.hitactor _outhit)))
    (Default|OpenDoor _asbp_door)))

(event EventBeginPlay
  (Input|AddMappingContext (PlayerController|LocalPlayerSubsystems|GetEnhancedInputLocalPlayerSubsystem) "/Game/Inputs/Action/imc_Player.imc_Player" 0 "(bIgnoreAllPressedKeysUntilRelease=True,bForceImmediately=False,bNotifyUserSettings=False)"))

(event EventTick
  (params (DeltaSeconds :type Float%20%28single-precision%29)))

(fn ConstructionScript)