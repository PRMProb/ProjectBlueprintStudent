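; Actor Blueprint that plays a hard-object drop sound when its Apple component's actor registers a hit.
; The Hit event passes a DoOnce with no reset, then a random switch plays the sound at the impact point on one of two outcomes.
; Volume scales with the magnitude of Apple's X velocity, clamped to full volume.
; The trailing zero Delay leads nowhere, and a duplicate sound node is unreachable.
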(event EventBeginPlay)

(event Collision|EventActorBeginOverlap
  (params (OtherActor :type Actor%20Object%20Reference)))

(event EventTick
  (params (DeltaSeconds :type Float%20%28single-precision%29)))

(event Collision|EventHit
  (params (MyComp :type Primitive%20Component%20Object%20Reference) (Other :type Actor%20Object%20Reference) (OtherComp :type Primitive%20Component%20Object%20Reference) (bSelfMoved :type Boolean) (HitLocation :type Vector :default "0, 0, 0") (HitNormal :type Vector :default "0, 0, 0") (NormalImpulse :type Vector :default "0, 0, 0") (Hit :type Hit%20Result%20Structure%20%28by%20ref%29))
  (Utilities|FlowControl|DoOnce false
    (:Completed
      (switch int (Math|Random|RandomInteger 2)
        (:0
          (Audio|PlaySoundatLocation "/Game/Audio/hard-object-drop-98768.hard-object-drop-98768" HitLocation "0, 0, 0" (Math|Float|Clamp(Float) (/ (Math|Vector|VectorLength (Math|Conversions|ToVector(Float) (.X (Math|Vector|BreakVector (Transformation|GetComponentVelocity (Variables|Default|GetApple)))))) 1e+01) 0.0 1.0) 1.0 0.0 0 0 0 0)
          (Utilities|FlowControl|Delay 0.0))))))

(fn ConstructionScript)